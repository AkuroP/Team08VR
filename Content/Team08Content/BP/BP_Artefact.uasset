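; BP_Artefact is an interactable collectible artefact that records its discovery in the game manager.
; On Interact it finds BP_GameManager, switches on its ArtefactNumber and sets the matching first, second or third found flag.
; It then destroys itself.
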(event EventInteract
  (bind _returnvalue (Actor|GetActorOfClass "/Game/Team08Content/BP/BP_GameManager.BP_GameManager_C"))
  (Variables|Default|SetGameManager _returnvalue)
  (switch int (Variables|Default|GetArtefactNumber)
    (:1
      (Variables|/Game/Team08Content/BP/BP_GameManager.BP_GameManager_C|SetFirstArtefactFound (Variables|Default|GetGameManager) true))
    (:2
      (Variables|/Game/Team08Content/BP/BP_GameManager.BP_GameManager_C|SetSecondArtefactFound (Variables|Default|GetGameManager) true))
    (:3
      (Variables|/Game/Team08Content/BP/BP_GameManager.BP_GameManager_C|SetThirdArtefactFound (Variables|Default|GetGameManager) true)))
  (Actor|DestroyActor))

(fn ConstructionScript)