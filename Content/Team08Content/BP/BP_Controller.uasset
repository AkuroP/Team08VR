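; Player controller that drives the BP_SubMarine actor from Enhanced Input in a VR game.
; BeginPlay adds IMC_Default, then caches the VR pawn and the submarine found in the level.
; IA_SubMarineMovement directly offsets the submarine's body collision along its forward vector and yaws it, without sweep or delta-time scaling.
; A disconnected force-and-torque version remains as a more realistic but less controllable alternative.
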(event Input|EnhancedActionEvents|EnhancedInputActionIA_SubMarineMovement
  (params (ActionValue :type Vector :default "0, 0, 0") (ElapsedSeconds :type Float%20%28double-precision%29) (TriggeredSeconds :type Float%20%28double-precision%29) (InputAction :type Input%20Action%20Object%20Reference :default "/Game/Team08Content/Input/IA_SubMarineMovement.IA_SubMarineMovement"))
  (bind _submarine (Variables|Default|GetSubMarine))
  (bind _submarine_bodycollision (Variables|/Game/Team08Content/BP/BP_SubMarine.BP_SubMarine_C|GetSubMarine_BodyCollision _submarine))
  ;[0 0 0] Sub Marine Move & Turn
  ;;[1 1 1] + contrôle, - réalisme
  (Transformation|AddRelativeLocation _submarine_bodycollision (* (Math|Vector|GetForwardVector _submarine_bodycollision) (.y ActionValue) (Variables|Default|GetSpeed)) false false)
  (Transformation|AddRelativeRotation _submarine_bodycollision (Math|Rotator|MakeRotator 0.0 0.0 (.x ActionValue)) false false))

(event EventBeginPlay
  (bind _returnvalue (PlayerController|LocalPlayerSubsystems|GetEnhancedInputLocalPlayerSubsystem))
  ;[0 0 0] IMC
  (Utilities|IsValid _returnvalue
    (:Is%20Valid
      (Input|AddMappingContext _returnvalue "/Game/VRTemplate/Input/IMC_Default.IMC_Default" 0 "(bIgnoreAllPressedKeysUntilRelease=True,bForceImmediately=False,bNotifyUserSettings=False)")
      (bind _asvrpawn (Utilities|Casting|CastToVRPawn (Game|Player|GetPlayerPawn 0)))
      (Variables|Default|SetVRPawn _asvrpawn)
      (bind _returnvalue_2 (Actor|GetActorOfClass "/Game/Team08Content/BP/BP_SubMarine.BP_SubMarine_C"))
      (Variables|Default|SetSubMarine _returnvalue_2))))

(event EventTick
  (params (DeltaSeconds :type Float%20%28single-precision%29)))

(fn ConstructionScript)