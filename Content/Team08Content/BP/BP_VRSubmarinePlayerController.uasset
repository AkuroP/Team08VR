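; BP_VRSubmarinePlayerController is the player controller for the VR submarine, firing a single light missile shortly after play begins.
; After a short delay on BeginPlay, it casts the first player's pawn to BP_VRSubmarine.
; It spawns BP_LightMissile at the LightMissileSpawn location using the camera's relative rotation.
; The missile's local-space velocity comes from its own speed times the camera's world forward vector.
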(event EventBeginPlay
  (Utilities|FlowControl|Delay 2.0)
  ;[1 0 0.1342] Shoot light missile
  (bind _asbp_vrsubmarine (Utilities|Casting|CastToBP_VRSubmarine (Pawn|GetControlledPawn (Game|GetPlayerController 0))))
  (bind _returnvalue (Game|SpawnActorfromClass "/Game/Team08Content/BP/BP_LightMissile.BP_LightMissile_C" (Math|Transform|MakeTransform (Transformation|GetWorldLocation (Variables|/Game/Team08Content/BP/BP_VRSubmarine.BP_VRSubmarine_C|GetLightMissileSpawn _asbp_vrsubmarine)) (Variables|/Script/Engine.SceneComponent|GetRelativeRotation (Variables|/Game/VRTemplate/Blueprints/VRPawn.VRPawn_C|GetCamera _asbp_vrsubmarine)) "1.000000,1.000000,1.000000") "Undefined" "MultiplyWithRoot" 0 0))
  (Game|Components|ProjectileMovement|SetVelocityinLocalSpace (Variables|/Game/Team08Content/BP/BP_LightMissile.BP_LightMissile_C|GetProjectileMovement _returnvalue) (* (Variables|/Game/Team08Content/BP/BP_LightMissile.BP_LightMissile_C|GetLightMissileSpeed _returnvalue) (Math|Vector|GetForwardVector (Variables|/Game/VRTemplate/Blueprints/VRPawn.VRPawn_C|GetCamera _asbp_vrsubmarine)))))

(fn ConstructionScript)